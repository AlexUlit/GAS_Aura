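; Fire Bolt gameplay ability that casts a projectile toward the location under the mouse.
; On activation it gets target data from the cursor hit and sends that location to the avatar as a warp target.
; It plays the cast montage while waiting for the Fire Bolt montage gameplay event.
; That event spawns the projectile toward the stored location, and the ability ends after a short delay.
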(event Ability|EventActivateAbility
  (bind _datahadnle (|TargetDataUnderMouse)
    (:ValidData
      (bind _output_get (Variables|Default|SetTargetLocation (.Location (Collision|BreakHitResult (Ability|TargetData|GetHitResultfromTargetData _datahadnle)))))
      (Class|CombatInterface|UpdateWarpTarget(Message) (Ability|GetAvatarActorfromActorInfo) _output_get)
      (|PlayMontageandWaitProxy "None" "/Game/Assets/Characters/Aura/Animations/Abilities/AM_Cast_FireBolt.AM_Cast_FireBolt" 1.0 "None" true 1.0 0.0 false
        (:then
          (Ability|Tasks|WaitGameplayEvent "(TagName=\"Event.Montage.FireBolt\")" 0
            (:EventReceived
              (Class|AuraProjectileSpell|SpawnProjectile (Variables|Default|GetTargetLocation))
              (Utilities|FlowControl|Delay 0.5)
              (Ability|EndAbility))))))))

(event Ability|EventOnEndAbility
  (params (bWasCancelled :type Boolean)))